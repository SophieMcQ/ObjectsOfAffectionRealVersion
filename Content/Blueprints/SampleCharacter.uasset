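; SampleCharacter is an interactable character that shows a dialogue widget with a new line on successive conversations.
; Interact toggles the widget: it removes an open one, or creates one, fills it with MyText and then calls GetCurrentText to queue the next line.
; GetCurrentText steps an index through four text variables and stays on the last, with BeginPlay priming the first.
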(event EventInteract
  (Utilities|IsValid (Variables|Default|GetDialogueWidget)
    (:Is%20Valid
      (Widget|RemovefromParent (Variables|Default|GetDialogueWidget))
      (Variables|Default|SetDialogueWidget 0))
    (:Is%20Not%20Valid
      (bind _returnvalue (UserInterface|CreateWidget "/Game/Blueprints/DialogueWidget.DialogueWidget_C" (Game|GetPlayerController 0)))
      (bind _output_get (Variables|Default|SetDialogueWidget _returnvalue))
      (UserInterface|Viewport|AddtoViewport _output_get 0)
      (Variables|/Game/Blueprints/DialogueWidget.DialogueWidget_C|SetDialogueText (Variables|Default|GetDialogueWidget) (Variables|Default|GetMyText))
      (CallFunction|GetCurrentText))))

(event EventBeginPlay
  (Variables|Default|Setindex 0)
  (CallFunction|GetCurrentText))

(fn ConstructionScript)

(fn GetCurrentText
  (switch int (Variables|Default|Getindex)
    (:0
      (Variables|Default|Setindex 1)
      (Variables|Default|SetMyText (Variables|Default|GetMyText_0)))
    (:1
      (Variables|Default|Setindex 2)
      (Variables|Default|SetMyText (Variables|Default|GetMyText_1)))
    (:2
      (Variables|Default|Setindex 3)
      (Variables|Default|SetMyText (Variables|Default|GetMyText_2)))
    (:3
      (Variables|Default|SetMyText (Variables|Default|GetMyText_3)))))