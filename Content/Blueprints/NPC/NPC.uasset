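; Interactable NPC that starts a dialogue through its AI controller.
; On BeginPlay it hands its DialogueTree to the NPCController that controls it.
; Interact tells that controller to start the dialogue, then sets DialogueFinished immediately after the call, with no completion callback.
; Both events do nothing if the AI controller is not an NPCController.
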(event EventInteract
  (bind _asnpccontroller (Utilities|Casting|CastToNPCController (AI|GetAIController self)))
  (Default|StartDialogue _asnpccontroller)
  (Variables|Default|SetDialogueFinished true))

(event EventBeginPlay
  (bind _asnpccontroller (Utilities|Casting|CastToNPCController (AI|GetAIController self)))
  (Variables|/Game/Blueprints/NPC/NPCController.NPCController_C|SetdialogueTree _asnpccontroller (Variables|Default|GetdialogueTree)))

(fn ConstructionScript)