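; AskQuestion is a behavior tree task that shows an NPC's question and its possible responses in the dialogue UI.
; On execute it reads the DialogueBox widget from the blackboard and sets its text to the question.
; It then adds a ResponseListUI to the box's overlay panel and fills it with one ResponsesUI widget per response.
; The task prints a debug string and never calls Finish Execute or handles a selection.
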(event EventReceiveExecuteAI
  (params (OwnerController :type AI%20Controller%20Object%20Reference) (ControlledPawn :type Pawn%20Object%20Reference))
  (bind _asdialogue_box (Utilities|Casting|CastToDialogueBox (Class|BTFunctionLibrary|GetBlackboardValueasObject (Variables|Default|GetBB_DialogueUI))))
  (bind _output_get (Variables|Default|SetDialogueBox _asdialogue_box))
  (Variables|/Game/Blueprints/NPC/DialogueBox.DialogueBox_C|SetdialogueText _output_get (Utilities|String|ToString(Text) (Variables|Default|GetQuestion)))
  (CallFunction|PrepareResponses)
  (Development|PrintString "Hello"))

(fn PrepareResponses
  (bind _returnvalue (UserInterface|CreateWidget "/Game/Blueprints/NPC/ResponseListUI.ResponseListUI_C"))
  (bind _output_get (Variables|Default|SetResponseListUI _returnvalue))
  (Class|Overlay|AddChildtoOverlay (Variables|/Game/Blueprints/NPC/DialogueBox.DialogueBox_C|GetResponseListPanel (Variables|Default|GetDialogueBox)) _output_get)
  (for _array_element (Variables|Default|GetResponses)
    (bind _returnvalue_2 (UserInterface|CreateWidget "/Game/Blueprints/NPC/ResponsesUI.ResponsesUI_C" 0 _array_element))
    (Class|VerticalBox|AddChildtoVerticalBox (Variables|/Game/Blueprints/NPC/ResponseListUI.ResponseListUI_C|GetResponseList (Variables|Default|GetResponseListUI)) _returnvalue_2)))