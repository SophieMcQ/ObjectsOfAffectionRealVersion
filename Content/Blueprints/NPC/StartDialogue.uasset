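; StartDialogue is a behavior tree task that opens NPC dialogue for the player.
; It makes the HUD's dialogue box visible through FirstPersonGameMode and stores that widget in a blackboard key.
; It then disables the player character's input, shows the mouse cursor and finishes with success.
; If the game mode cast fails, it stops without calling FinishExecute.
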(event EventReceiveExecuteAI
  (params (OwnerController :type AI%20Controller%20Object%20Reference) (ControlledPawn :type Pawn%20Object%20Reference))
  (bind _returnvalue (Game|GetPlayerController 0))
  (bind _asfirst_person_game_mode (Utilities|Casting|CastToFirstPersonGameMode (Game|GetGameMode)))
  (Widget|SetVisibility (Variables|/Game/Blueprints/NPC/HeadsUpDisplay.HeadsUpDisplay_C|GetDialogueBox (Variables|/Game/FirstPersonBP/Blueprints/FirstPersonGameMode.FirstPersonGameMode_C|GetHeadsUpDisplay _asfirst_person_game_mode)) "Visible")
  (Class|BTFunctionLibrary|SetBlackboardValueasObject (Variables|Default|GetBB_DialogueUI) (Variables|/Game/Blueprints/NPC/HeadsUpDisplay.HeadsUpDisplay_C|GetDialogueBox (Variables|/Game/FirstPersonBP/Blueprints/FirstPersonGameMode.FirstPersonGameMode_C|GetHeadsUpDisplay _asfirst_person_game_mode)))
  (Input|DisableInput (Game|GetPlayerCharacter 0) _returnvalue)
  (Variables|/Script/Engine.PlayerController|SetbShowMouseCursor _returnvalue true)
  (AI|BehaviorTree|FinishExecute true))