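; Behavior tree task that ends an NPC dialogue and returns control to the player.
; On execute, it hides the dialogue widget stored on the blackboard and tells the NPC controller to end the dialogue.
; It then hides the mouse cursor, re-enables player character input, finishes successfully and plays a tap sound.
; A failed cast stops execution without finishing the task.
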(event EventReceiveExecuteAI
  (params (OwnerController :type AI%20Controller%20Object%20Reference) (ControlledPawn :type Pawn%20Object%20Reference))
  (bind _returnvalue (Game|GetPlayerController 0))
  (bind _aswidget (Utilities|Casting|CastToWidget (Class|BTFunctionLibrary|GetBlackboardValueasObject (Variables|Default|GetBB_DialogueUI))))
  (Widget|SetVisibility _aswidget "Hidden")
  (bind _asnpccontroller (Utilities|Casting|CastToNPCController OwnerController))
  (Default|EndDialogue _asnpccontroller)
  (Variables|/Script/Engine.PlayerController|SetbShowMouseCursor _returnvalue false)
  (Input|EnableInput (Game|GetPlayerCharacter 0) _returnvalue)
  (AI|BehaviorTree|FinishExecute true)
  (Audio|PlaySound2D "/Game/Sounds/tapSound.tapSound" 1.0 1.0 0.0 0 0))