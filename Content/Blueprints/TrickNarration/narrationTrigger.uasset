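; A one-shot narration trigger that shows a sequence of dialogue lines when something overlaps its Trigger component.
; DisplayText creates a DialogueWidget for the current TextList entry, waits DelayTime, removes all dialogue widgets, then calls itself for the next entry.
; After the last line it re-enables player character input, though nothing here disables it.
; An unconnected single-line version of the display logic remains unused.
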(event OnComponentBeginOverlap(trigger)
  (params (OverlappedComponent :type Primitive%20Component%20Object%20Reference) (OtherActor :type Actor%20Object%20Reference) (OtherComp :type Primitive%20Component%20Object%20Reference) (OtherBodyIndex :type Integer) (bFromSweep :type Boolean) (SweepResult :type Hit%20Result%20Structure%20%28by%20ref%29))
  (if (not (Variables|Default|GethasFinished))
    (Variables|Default|SetphrasesLength (Utilities|Array|Length (Variables|Default|GettextList)))
    (CallFunction|DisplayText)
    (Variables|Default|SethasFinished true)))

(event Custom|DisplayText
  (bind _returnvalue (UserInterface|CreateWidget "/Game/Blueprints/BasicDialogue/DialogueWidget.DialogueWidget_C"))
  (Variables|/Game/Blueprints/BasicDialogue/DialogueWidget.DialogueWidget_C|SetDialogueText _returnvalue (Utilities|Array|Get(acopy) (Variables|Default|GettextList) (Variables|Default|Getindex)))
  (UserInterface|Viewport|AddtoViewport _returnvalue 0)
  (Utilities|FlowControl|Delay (Variables|Default|GetdelayTime))
  (bind _foundwidgets (Widget|GetAllWidgetsOfClass "/Game/Blueprints/BasicDialogue/DialogueWidget.DialogueWidget_C" true))
  (Widget|RemovefromParent _foundwidgets)
  (if (< (+ (Variables|Default|Getindex) 1) (Variables|Default|GetphrasesLength))
    (Variables|Default|Setindex (+ (Variables|Default|Getindex) 1))
    (CallFunction|DisplayText)
    (else
      (Input|EnableInput (Game|GetPlayerCharacter 0) 0))))

(event EventBeginPlay)

(fn ConstructionScript)