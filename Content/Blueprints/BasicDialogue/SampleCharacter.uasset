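; Sample dialogue character that creates a hidden dialogue widget at BeginPlay and fills it with its dialogue and choice text.
; Interact toggles the widget and, when showing it, calls GetCurrentText, which switches on State.
; Only state 0 is handled: State1 calls NoChoice on the widget and sets the character's DialogueText to MyText1.
; Choice events record PlayerChoiceVar while the widget is visible, but nothing here reads it or advances State.
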(event EventChoice1
  (if (Widget|IsVisible (Variables|Default|GetDialogueWidget))
    (Variables|Default|SetplayerChoiceVar 1)))

(event EventChoice2
  (if (Widget|IsVisible (Variables|Default|GetDialogueWidget))
    (Variables|Default|SetplayerChoiceVar 2)))

(event EventInteract
  (bind _dialoguewidget (Variables|Default|GetDialogueWidget))
  (if (Widget|IsVisible _dialoguewidget)
    (Widget|SetVisibility _dialoguewidget "Hidden")
    (else
      (Widget|SetVisibility _dialoguewidget "Visible")
      (CallFunction|GetCurrentText))))

(event EventBeginPlay
  (bind _returnvalue (UserInterface|CreateWidget "/Game/Blueprints/BasicDialogue/DialogueWidget.DialogueWidget_C" (Game|GetPlayerController 0)))
  (bind _output_get (Variables|Default|SetDialogueWidget _returnvalue))
  (UserInterface|Viewport|AddtoViewport _output_get 0)
  (Widget|SetVisibility (Variables|Default|GetDialogueWidget) "Hidden")
  (Variables|Default|SetState 0)
  (Variables|/Game/Blueprints/BasicDialogue/DialogueWidget.DialogueWidget_C|SetDialogueText (Variables|Default|GetDialogueWidget) (Variables|Default|GetDialogueText))
  (Variables|/Game/Blueprints/BasicDialogue/DialogueWidget.DialogueWidget_C|SetChoice1 (Variables|Default|GetDialogueWidget) (Variables|Default|GetChoice1Text))
  (Variables|/Game/Blueprints/BasicDialogue/DialogueWidget.DialogueWidget_C|SetChoice2 (Variables|Default|GetDialogueWidget) (Variables|Default|GetChoice2Text))
  (Variables|/Game/Blueprints/BasicDialogue/DialogueWidget.DialogueWidget_C|SetDefaultChoice (Variables|Default|GetDialogueWidget) (Variables|Default|GetDefaultTextChoice)))

(fn ConstructionScript)

(fn GetCurrentText
  (switch int (Variables|Default|GetState)
    (:0
      (CallFunction|State1))))

(fn State1
  (Default|NoChoice (Variables|Default|GetDialogueWidget))
  (Variables|Default|SetDialogueText (Variables|Default|GetMyText_1)))