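; A door Blueprint that the player toggles with the left mouse button, swinging it with a timeline.
; Overlapping the FrontCollision component enables input on the actor, and leaving it disables input.
; Each click plays the DoorOpenclose timeline forward or in reverse, driving the door's relative yaw.
; The Front flag is set on overlap but never read, so the swing ignores the player's side.
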(event OnComponentBeginOverlap(FrontCollision)
  (params (OverlappedComponent :type Primitive%20Component%20Object%20Reference) (OtherActor :type Actor%20Object%20Reference) (OtherComp :type Primitive%20Component%20Object%20Reference) (OtherBodyIndex :type Integer) (bFromSweep :type Boolean) (SweepResult :type Hit%20Result%20Structure%20%28by%20ref%29))
  ;[1 1 1] EnableInput
  (Input|EnableInput (Game|GetPlayerController 0))
  (Variables|Default|Setfront true))

(event OnComponentEndOverlap(FrontCollision)
  (params (OverlappedComponent :type Primitive%20Component%20Object%20Reference) (OtherActor :type Actor%20Object%20Reference) (OtherComp :type Primitive%20Component%20Object%20Reference) (OtherBodyIndex :type Integer))
  ;[1 1 1] EnableInput
  (Input|DisableInput (Game|GetPlayerController 0)))

(event EventBeginPlay
  (Variables|Default|SetdoorClosed false))

(event Input|MouseEvents|LeftMouseButton
  (params (Key :type Key%20Structure :default "None"))
  ;[1 1 1] Door opens depending on location of player
  (:Pressed
    (if (Variables|Default|GetdoorClosed)
      (Variables|Default|SetdoorClosed false)
      (bind _door_open_close (Timeline|Door%20open/close ReverseFromEnd)
        (:Update
          (Transformation|SetRelativeRotation (Variables|Default|GetDoor) (Math|Rotator|MakeRotator 0.0 0.0 _door_open_close) false false)))
      (else
        (Variables|Default|SetdoorClosed true)
        (Timeline|Door%20open/close PlayFromStart)))))

(fn ConstructionScript)